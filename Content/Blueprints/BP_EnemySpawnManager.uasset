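; BP_EnemySpawnManager scatters the BP_NewEnemy actors already in the level at random positions when play begins, without spawning any.
; On BeginPlay it gathers them and, if the game mode is InGameMode, runs one downward visibility trace per enemy.
; Trace start and end X/Y are randomized independently within a fixed area, so traces slant.
; Enemies teleport-free move to the impact point without sweep; a miss leaves them in place.
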(event EventBeginPlay
  (bind _returnvalue (Math|Random|RandomIntegerinRange -23650 -2640))
  (bind _returnvalue_2 (Math|Random|RandomIntegerinRange -2450 28260))
  (bind _outactors (Actor|GetAllActorsOfClass "/Game/Blueprints/BP_NewEnemy.BP_NewEnemy_C"))
  (Variables|Default|SetEnemyArr _outactors)
  (Utilities|Casting|CastToInGameMode (Game|GetGameMode))
  (for _array_element (Variables|Default|GetEnemyArr)
    (bind (_outhit _returnvalue_3) (Collision|LineTraceByChannel (Math|Vector|MakeVector (Math|Conversions|ToFloat(Integer) _returnvalue) (Math|Conversions|ToFloat(Integer) _returnvalue_2) 6e+03) (Math|Vector|MakeVector (Math|Conversions|ToFloat(Integer) _returnvalue) (Math|Conversions|ToFloat(Integer) _returnvalue_2) -8e+03) "TraceTypeQuery1" false 0 "None"))
    (if _returnvalue_3
      (Transformation|SetActorLocation _array_element (.impactpoint _outhit) false false))))

(fn ConstructionScript)