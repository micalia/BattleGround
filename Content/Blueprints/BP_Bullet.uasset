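; BP_Bullet is a projectile actor that damages enemies it overlaps and removes itself after a set lifetime.
; On overlap it casts the other actor to Enemy and subtracts a fixed amount directly from its CurrHP, without destroying the bullet.
; Tick accumulates delta time in CurrTime and destroys the actor once it exceeds SetTime.
; The graphs contain no movement logic.
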(event EventBeginPlay)

(event Collision|EventActorBeginOverlap
  (params (OtherActor :type Actor%20Object%20Reference))
  (bind _asenemy (Utilities|Casting|CastToEnemy OtherActor))
  (Variables|/Script/BattleGround.Enemy|SetcurrHP _asenemy (- (Variables|/Script/BattleGround.Enemy|GetcurrHP _asenemy) (Math|Float|MakeLiteralFloat 1.0))))

(event EventTick
  (params (DeltaSeconds :type Float%20%28single-precision%29))
  (bind _output_get (Variables|Default|SetcurrTime (+ DeltaSeconds (Variables|Default|GetcurrTime))))
  (if (> _output_get (Variables|Default|GetsetTime))
    (Actor|DestroyActor)))

(fn ConstructionScript)