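; Item spawner actor that scatters random pickups from SpawnItems across the map at BeginPlay, only when the game mode is InGameMode.
; Each loop over SpawnItemCount runs a Visibility line trace from high to low within hard-coded XY bounds, spawning an item at the impact point.
; Trace start and end XY are randomized independently, so traces slant, and hits are not checked.
; An older fixed-height, two-region spawn branch remains unconnected.
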(event EventBeginPlay
  (bind _returnvalue (Math|Random|RandomIntegerinRange -23650 -2640))
  (bind _returnvalue_2 (Math|Random|RandomIntegerinRange -2450 28260))
  (Utilities|Casting|CastToInGameMode (Game|GetGameMode))
  (for _index (range 0 (Variables|Default|GetSpawnItemCount))
    (bind _outhit (Collision|LineTraceByChannel (Math|Vector|MakeVector (Math|Conversions|ToFloat(Integer) _returnvalue) (Math|Conversions|ToFloat(Integer) _returnvalue_2) 6e+03) (Math|Vector|MakeVector (Math|Conversions|ToFloat(Integer) _returnvalue) (Math|Conversions|ToFloat(Integer) _returnvalue_2) -8e+03) "TraceTypeQuery1" false 0 "None"))
    (Game|SpawnActorfromClass (.OutItem (Utilities|Array|Random (Variables|Default|GetSpawnItems))) (Math|Transform|MakeTransform (.impactpoint _outhit) "0, 0, 0" "1.000000,1.000000,1.000000") "Undefined" "MultiplyWithRoot" 0 0)))

(event Collision|EventActorBeginOverlap
  (params (OtherActor :type Actor%20Object%20Reference)))

(event EventTick
  (params (DeltaSeconds :type Float%20%28single-precision%29)))

(fn ConstructionScript)