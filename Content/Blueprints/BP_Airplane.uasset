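; BP_Airplane is an airplane actor that flies in a straight line along the world X axis.
; BeginPlay sets Direction to positive X and prints the starting location to the screen.
; Tick adds Direction times Speed times delta seconds to the actor location each frame, without sweeping for collision.
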(event EventBeginPlay
  (Variables|Default|SetDirection "1.000000,0.000000,0.000000")
  (Development|PrintString (Utilities|String|ToString(Vector) (Transformation|GetActorLocation))))

(event Collision|EventActorBeginOverlap
  (params (OtherActor :type Actor%20Object%20Reference)))

(event EventTick
  (params (DeltaSeconds :type Float%20%28single-precision%29))
  (Transformation|SetActorLocation (+ (Transformation|GetActorLocation) (* DeltaSeconds (* (Variables|Default|GetSpeed) (Variables|Default|GetDirection)))) false false))

(fn ConstructionScript)