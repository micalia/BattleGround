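; BP_NewEnemy is an enemy Blueprint whose health drains while it is outside what its flag treats as a magnetic area.
; BeginPlay seeds BPCurrHP from FullHp, and any actor overlap toggles IsInMagnetic, with a debug print when an overlap ends.
; Tick subtracts a fixed amount from BPCurrHP while the flag is off, so the drain scales with frame rate.
; The graph has no lower clamp or death handling.
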(event Collision|EventActorBeginOverlap
  (params (OtherActor :type Actor%20Object%20Reference))
  (Variables|Default|SetIsInMagnetic? true))

(event EventTick
  (params (DeltaSeconds :type Float%20%28single-precision%29))
  (if (not (Variables|Default|GetIsInMagnetic?))
    (Variables|Default|SetBP_CurrHP (- (Variables|Default|GetBP_CurrHP) 0.05))))

(event Collision|EventActorEndOverlap
  (params (OtherActor :type Actor%20Object%20Reference))
  (Variables|Default|SetIsInMagnetic? false)
  (Development|PrintString "EnemyIsInMag"))

(event EventBeginPlay
  (Variables|Default|SetBP_CurrHP (Math|Conversions|ToFloat(Integer) (Variables|Default|GetFullHp))))

(fn ConstructionScript)