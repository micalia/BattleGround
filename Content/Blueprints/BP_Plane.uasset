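; BP_Plane is an actor that flies in a straight line from a random outlying start point toward a flag.
; On BeginPlay it picks a start position on one of four lines through chained random rolls, moves BP_flag to a random spot, then turns to face it.
; It stores that normalized direction once, and Tick moves it by Speed and delta time without sweeping or stopping at the flag.
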(event EventBeginPlay
  (bind _returnvalue (Math|Random|RandomIntegerinRange 0 3))
  (bind _returnvalue_2 (Math|Random|RandomFloatinRange -1e+03 4e+03))
  (if (== _returnvalue 0)
    (Variables|Default|Setx -1e+03)
    (Variables|Default|Sety _returnvalue_2)
    (elif (== _returnvalue 1)
      (Variables|Default|Setx 5e+03)
      (Variables|Default|Sety _returnvalue_2)
      (elif (== _returnvalue 2)
        (Variables|Default|Setx _returnvalue_2)
        (Variables|Default|Sety -1e+03)
        (else
          (Variables|Default|Setx _returnvalue_2)
          (Variables|Default|Sety -5e+03)))))
  (Transformation|SetActorLocation (Math|Vector|MakeVector (Variables|Default|Getx) (Variables|Default|Gety) (Variables|Default|Getz)) false false)
  (bind _returnvalue_3 (Actor|GetActorOfClass "/Game/Blueprints/BP_flag.BP_flag_C"))
  (Transformation|SetActorLocation _returnvalue_3 (Math|Vector|MakeVector (Math|Random|RandomFloatinRange 7e+02 2e+03) (Math|Random|RandomFloatinRange 5e+02 2.5e+03) (Variables|Default|Getz)) false false)
  (bind _returnvalue_4 (Actor|GetActorOfClass "/Game/Blueprints/BP_flag.BP_flag_C"))
  (Variables|Default|SetDirection (Math|Vector|Normalize (- (Transformation|GetActorLocation _returnvalue_4) (Transformation|GetActorLocation))))
  (Transformation|SetActorRotation (Math|Rotator|FindLookatRotation (Transformation|GetActorLocation) (Transformation|GetActorLocation _returnvalue_4))))

(event Collision|EventActorBeginOverlap
  (params (OtherActor :type Actor%20Object%20Reference)))

(event EventTick
  (params (DeltaSeconds :type Float%20%28single-precision%29))
  (Transformation|SetActorLocation (+ (Transformation|GetActorLocation) (* DeltaSeconds (* (Variables|Default|GetSpeed) (Variables|Default|GetDirection)))) false false))

(fn ConstructionScript)